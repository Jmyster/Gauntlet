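; Player character with four selectable classes (Warrior, Elf, Wizard, Valkyrie), Enhanced Input movement, projectile shooting and potion attacks.
; Pausing toggles the class selector widget, which holds a reference to this character; SetVariablesBasedOnClass writes the chosen class's stats into PlayerData and prints them.
; Shooting passes shot damage to the projectile and stays locked until it is destroyed, allowing one shot at a time.
; Potion throws require Potions above zero; death only prints a message.
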(event OnPlayerDeath(PlayerData)
  ;[0.2188 0.2188 0.2188] On player death
  (Development|PrintString "You Died"))

(event Custom|SetVariablesBasedOnClass
  (bind _classtype (Variables|Default|GetClassType))
  ;[0.1927 0.1927 0.1927] Set player stats based on class
  (if (Utilities|Enum|Equal(Enum) _classtype "NewEnumerator0")
    (CallFunction|WarriorStats)
    (Utilities|PrintStats)
    (elif (Utilities|Enum|Equal(Enum) _classtype "NewEnumerator1")
      (CallFunction|ElfStats)
      (Utilities|PrintStats)
      (elif (Utilities|Enum|Equal(Enum) _classtype "NewEnumerator2")
        (CallFunction|WizardStats)
        (Utilities|PrintStats)
        (elif (Utilities|Enum|Equal(Enum) _classtype "NewEnumerator3")
          (CallFunction|ValkyrieStats)
          (Utilities|PrintStats))))))

(event Custom|OnProjectileDestroyed
  (params (DestroyedActor :type Actor%20Object%20Reference))
  ;[0.1667 0.1667 0.1667] Shoot
  (Variables|Default|SetCanShoot true)
  (Development|PrintString "Can shoot"))

(event Input|EnhancedActionEvents|EnhancedInputActionIA_Shoot
  (params (ActionValue :type Boolean) (ElapsedSeconds :type Float%20%28double-precision%29) (TriggeredSeconds :type Float%20%28double-precision%29) (InputAction :type Input%20Action%20Object%20Reference :default "/Game/Jonathan_Sullivan/Blueprints/Controls/IA_Shoot.IA_Shoot"))
  (bind _returnvalue (Transformation|GetActorTransform))
  ;[0.1667 0.1667 0.1667] Shoot
  (:Triggered
    (if (Variables|Default|GetCanShoot)
      (Variables|Default|SetCanShoot false)
      (bind _returnvalue_2 (Game|SpawnActorfromClass "/Game/Jonathan_Sullivan/Blueprints/BP_Projectile.BP_Projectile_C" (Math|Transform|MakeTransform (.location _returnvalue) (.rotation _returnvalue) "1.000000,1.000000,1.000000") "Undefined" 0 0))
      (bind _output_get (Variables|Default|SetSpawnedProj _returnvalue_2))
      (Game|BindEventtoOnDestroyed _output_get (delegate Custom|OnProjectileDestroyed))
      (Variables|/Game/Jonathan_Sullivan/Blueprints/BP_Projectile.BP_Projectile_C|SetDamage _output_get (Variables|/Script/Gauntlet.PlayerData|GetShotDamagePower (Variables|Default|GetPlayerData))))))

(event Input|EnhancedActionEvents|EnhancedInputActionIA_MagicAttack
  (params (ActionValue :type Boolean) (ElapsedSeconds :type Float%20%28double-precision%29) (TriggeredSeconds :type Float%20%28double-precision%29) (InputAction :type Input%20Action%20Object%20Reference :default "/Game/Jonathan_Sullivan/Blueprints/Controls/IA_MagicAttack.IA_MagicAttack"))
  (bind _returnvalue (Transformation|GetActorTransform))
  ;[0.2135 0.2135 0.2135] Potion Attack
  (:Triggered
    (if (> (Variables|Default|GetPotions) 0)
      (Game|SpawnActorfromClass "/Game/Jonathan_Sullivan/Blueprints/BP_Potion.BP_Potion_C" (Math|Transform|MakeTransform (.location _returnvalue) (.rotation _returnvalue) "1.000000,1.000000,1.000000") "Undefined" 0 0)
      (else
        (Development|PrintString "Need more potions")))))

(event Input|EnhancedActionEvents|EnhancedInputActionIA_Right-Left
  (params (ActionValue :type Float%20%28double-precision%29) (ElapsedSeconds :type Float%20%28double-precision%29) (TriggeredSeconds :type Float%20%28double-precision%29) (InputAction :type Input%20Action%20Object%20Reference :default "/Game/Jonathan_Sullivan/Blueprints/Controls/IA_Right-Left.IA_Right-Left"))
  (bind _returnvalue (Pawn|GetControlRotation :!class /Script/Engine.Pawn))
  ;[0.08333 0.08333 0.08333] Movement Controls
  (:Triggered
    (Pawn|Input|AddMovementInput (Math|Vector|GetRightVector (Math|Rotator|MakeRotator (.roll _returnvalue) 0.0 (.yaw _returnvalue))) ActionValue false)))

(event Input|EnhancedActionEvents|EnhancedInputActionIA_Forwards-Backwards
  (params (ActionValue :type Float%20%28double-precision%29) (ElapsedSeconds :type Float%20%28double-precision%29) (TriggeredSeconds :type Float%20%28double-precision%29) (InputAction :type Input%20Action%20Object%20Reference :default "/Game/Jonathan_Sullivan/Blueprints/Controls/IA_Forwards-Backwards.IA_Forwards-Backwards"))
  ;[0.08333 0.08333 0.08333] Movement Controls
  (:Triggered
    (Pawn|Input|AddMovementInput (Math|Vector|GetForwardVector (Math|Rotator|MakeRotator 0.0 0.0 (.yaw (Pawn|GetControlRotation :!class /Script/Engine.Pawn)))) ActionValue false)))

(event Input|EnhancedActionEvents|EnhancedInputActionIA_Pause
  (params (ActionValue :type Boolean) (ElapsedSeconds :type Float%20%28double-precision%29) (TriggeredSeconds :type Float%20%28double-precision%29) (InputAction :type Input%20Action%20Object%20Reference :default "/Game/Jonathan_Sullivan/Blueprints/Controls/IA_Pause.IA_Pause"))
  (bind _returnvalue (Game|IsGamePaused))
  (bind _returnvalue_2 (Game|GetPlayerController 0))
  (bind _class_selector_ui (Variables|Default|GetClass%20Selector%20UI))
  (:Triggered
    (Game|SetGamePaused (not _returnvalue))
    (if _returnvalue
      (UserInterface|Viewport|AddtoViewport _class_selector_ui 0)
      (Variables|/Script/Engine.PlayerController|SetbShowMouseCursor _returnvalue_2 true)
      (else
        (Widget|RemovefromParent _class_selector_ui)
        (Variables|/Script/Engine.PlayerController|SetbShowMouseCursor _returnvalue_2 false)))))

(event EventBeginPlay
  (bind _asplayer_controller (Utilities|Casting|CastToPlayerController (Pawn|GetController)))
  (Input|AddMappingContext (PlayerController|LocalPlayerSubsystems|GetEnhancedInputLocalPlayerSubsystem _asplayer_controller) "/Game/Jonathan_Sullivan/Blueprints/Controls/IM_Controls.IM_Controls" 0 "(bIgnoreAllPressedKeysUntilRelease=True,bForceImmediately=False)")
  (bind _returnvalue (UserInterface|CreateWidget "/Game/Jonathan_Sullivan/Blueprints/UI/WBP_ClassSelector.WBP_ClassSelector_C"))
  (bind _output_get (Variables|Default|SetClass%20Selector%20UI _returnvalue))
  (Variables|/Game/Jonathan_Sullivan/Blueprints/UI/WBP_ClassSelector.WBP_ClassSelector_C|SetBP_Character _output_get self))

(fn ConstructionScript)

(fn WarriorStats
  (bind _playerdata (Variables|Default|GetPlayerData))
  (Variables|/Script/Gauntlet.PlayerData|SetPlayerHealth _playerdata 700)
  (Variables|/Script/Gauntlet.PlayerData|SetPlayerArmor _playerdata 90)
  (Variables|/Script/Gauntlet.PlayerData|SetPlayerSpeed _playerdata 70)
  (Variables|/Script/Gauntlet.PlayerData|SetDamagePower _playerdata 5e+01)
  (Variables|/Script/Gauntlet.PlayerData|SetShotDamagePower _playerdata 2e+01)
  (Variables|/Script/Gauntlet.PlayerData|SetAttackSpeed _playerdata 1.0)
  (Variables|/Script/Gauntlet.PlayerData|SetMagicPower _playerdata 2.0)
  (Variables|/Script/Gauntlet.PlayerData|SetShotSpeed _playerdata 1.0))

(fn ElfStats
  (bind _playerdata (Variables|Default|GetPlayerData))
  (Variables|/Script/Gauntlet.PlayerData|SetPlayerHealth _playerdata 700)
  (Variables|/Script/Gauntlet.PlayerData|SetPlayerArmor _playerdata 70)
  (Variables|/Script/Gauntlet.PlayerData|SetPlayerSpeed _playerdata 120)
  (Variables|/Script/Gauntlet.PlayerData|SetDamagePower _playerdata 2e+01)
  (Variables|/Script/Gauntlet.PlayerData|SetShotDamagePower _playerdata 5e+01)
  (Variables|/Script/Gauntlet.PlayerData|SetAttackSpeed _playerdata 1.5)
  (Variables|/Script/Gauntlet.PlayerData|SetMagicPower _playerdata 4e+01)
  (Variables|/Script/Gauntlet.PlayerData|SetShotSpeed _playerdata 1.6))

(fn WizardStats
  (bind _playerdata (Variables|Default|GetPlayerData))
  (Variables|/Script/Gauntlet.PlayerData|SetPlayerHealth _playerdata 700)
  (Variables|/Script/Gauntlet.PlayerData|SetPlayerArmor _playerdata 60)
  (Variables|/Script/Gauntlet.PlayerData|SetPlayerSpeed _playerdata 60)
  (Variables|/Script/Gauntlet.PlayerData|SetDamagePower _playerdata 1e+01)
  (Variables|/Script/Gauntlet.PlayerData|SetShotDamagePower _playerdata 2e+01)
  (Variables|/Script/Gauntlet.PlayerData|SetAttackSpeed _playerdata 1.4)
  (Variables|/Script/Gauntlet.PlayerData|SetMagicPower _playerdata 5e+01)
  (Variables|/Script/Gauntlet.PlayerData|SetShotSpeed _playerdata 1.0))

(fn ValkyrieStats
  (bind _playerdata (Variables|Default|GetPlayerData))
  (Variables|/Script/Gauntlet.PlayerData|SetPlayerHealth _playerdata 700)
  (Variables|/Script/Gauntlet.PlayerData|SetPlayerArmor _playerdata 110)
  (Variables|/Script/Gauntlet.PlayerData|SetPlayerSpeed _playerdata 90)
  (Variables|/Script/Gauntlet.PlayerData|SetDamagePower _playerdata 4e+01)
  (Variables|/Script/Gauntlet.PlayerData|SetShotDamagePower _playerdata 1e+01)
  (Variables|/Script/Gauntlet.PlayerData|SetAttackSpeed _playerdata 1.0)
  (Variables|/Script/Gauntlet.PlayerData|SetMagicPower _playerdata 5.0)
  (Variables|/Script/Gauntlet.PlayerData|SetShotSpeed _playerdata 1.3))