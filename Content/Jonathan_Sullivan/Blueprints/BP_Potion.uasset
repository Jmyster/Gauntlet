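; BP_Potion is a thrown potion projectile that deals area damage to enemies.
; On BeginPlay a Launch timeline moves it forward with sweep, then a ScaleOverTime timeline grows its Sphere before the actor destroys itself.
; Begin and end overlap events maintain a list of overlapping actors, and on Destroyed it applies Damage to each BaseEnemy in that list.
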(event EventBeginPlay
  (bind _returnvalue (Transformation|GetActorTransform))
  (bind _sphere (Variables|Default|GetSphere))
  (bind _returnvalue_2 (Transformation|GetWorldScale _sphere))
  ;[0.1771 0.1771 0.1771] Launch Physics
  (bind _alpha (Timeline|Launch Play)
    (:Update
      (Transformation|SetActorLocation (Math|Vector|Lerp(Vector) (.location _returnvalue) (+ (.location _returnvalue) (* (Math|Vector|GetForwardVector (.rotation _returnvalue)) "5.000000,5.000000,5.000000")) _alpha) true false))
    (:Finished
      (Variables|Default|SetCanHit true)
      (bind _alpha_2 (Timeline|ScaleOverTime PlayFromStart)
        (:Update
          (Transformation|SetRelativeScale3D (Variables|Default|GetSphere) (Math|Vector|Lerp(Vector) _returnvalue_2 (* _returnvalue_2 "1.200000,1.200000,1.200000") _alpha_2)))
        (:Finished
          (Actor|DestroyActor))))))

(event Collision|EventActorBeginOverlap
  (params (OtherActor :type Actor%20Object%20Reference))
  (bind _overlappingactors (Variables|Default|GetOverLappingActors))
  (if (not (Utilities|Array|ContainsItem _overlappingactors OtherActor))
    (Utilities|Array|Add _overlappingactors OtherActor)))

(event Collision|EventActorEndOverlap
  (params (OtherActor :type Actor%20Object%20Reference))
  (bind _overlappingactors (Variables|Default|GetOverLappingActors))
  (if (Utilities|Array|ContainsItem _overlappingactors OtherActor)
    (Utilities|Array|RemoveItem _overlappingactors OtherActor)))

(event EventDestroyed
  (for _array_element (Variables|Default|GetOverLappingActors)
    (bind _asbase_enemy (Utilities|Casting|CastToBaseEnemy _array_element))
    (Class|BaseEnemy|ReceiveDamage _asbase_enemy (Variables|Default|GetDamage))))

(fn ConstructionScript)